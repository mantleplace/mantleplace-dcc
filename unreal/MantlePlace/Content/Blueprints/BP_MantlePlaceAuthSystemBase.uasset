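; MantlePlace auth system Blueprint that reports authentication events as debug prints.
; It handles sign-in results, token refresh, sign-out completion and auth state changes, printing the incoming message or a fixed status string.
; State changes switch over the auth state enum to print its name.
; The graph holds only this logging, with no sign-in or token logic of its own.
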(event `self.OnSignInResult`
  (params (bSuccess :type Boolean) (Message :type String))
  (`KismetSystemLibrary.PrintString` null Message))

(event `self.OnTokenRefreshed`
  (params (bSuccess :type Boolean))
  (`KismetSystemLibrary.PrintString` null (select `bool` bSuccess :`false` "Auth: token refresh failed" :`true` "Auth: token refreshed")))

(event `self.OnSignOutComplete`
  (`KismetSystemLibrary.PrintString` null "Auth: signed out"))

(event `self.OnAuthStateChanged`
  (params (NewState :type "EMantlePlaceAuthState Enum" :default "Unauthenticated"))
  (switch `EMantlePlaceAuthState` NewState
    (:`Unauthenticated`
      (`KismetSystemLibrary.PrintString` null "Auth state: Unauthenticated"))
    (:`Authenticating`
      (`KismetSystemLibrary.PrintString` null "Auth state: Authenticating"))
    (:`Authenticated`
      (`KismetSystemLibrary.PrintString` null "Auth state: Authenticated"))
    (:`Refreshing`
      (`KismetSystemLibrary.PrintString` null "Auth state: Refreshing"))
    (:`Failed`
      (`KismetSystemLibrary.PrintString` null "Auth state: Failed"))))